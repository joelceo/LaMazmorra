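; Dungeon gate actor that swings open on its pivot when any actor overlaps its trigger box.
; Overlap plays the OpenDoor timeline, which increments DoorOpenAngle by a fixed step per update, so the swing speed depends on frame rate.
; Tick and the construction script apply that angle, clamped and negated, as GatePivot's relative yaw.
; A barrel cast is left unconnected, and no closing logic exists.
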(event OnComponentBeginOverlap(Box)
  (params (OverlappedComponent :type Primitive%20Component%20Object%20Reference) (OtherActor :type Actor%20Object%20Reference) (OtherComp :type Primitive%20Component%20Object%20Reference) (OtherBodyIndex :type Integer) (bFromSweep :type Boolean) (SweepResult :type Hit%20Result%20Structure%20%28by%20ref%29))
  (Timeline|Open%20Door Play
    (:Update
      (Variables|Default|SetDoor%20Open%20Angle (+ (Variables|Default|GetDoor%20Open%20Angle) 1.0)))))

(event EventBeginPlay)

(event EventTick
  (params (DeltaSeconds :type Float%20%28single-precision%29))
  (Transformation|SetRelativeRotation (Variables|Default|GetGatePivot) (Math|Rotator|MakeRotator 0.0 0.0 (* (Math|Float|Clamp(Float) (Variables|Default|GetDoor%20Open%20Angle) 0.0 1.2e+02) -1.0)) false false))

(fn ConstructionScript
  (Transformation|SetRelativeRotation (Variables|Default|GetGatePivot) (Math|Rotator|MakeRotator 0.0 0.0 (* (Math|Float|Clamp(Float) (Variables|Default|GetDoor%20Open%20Angle) 0.0 1.2e+02) -1.0)) false false))